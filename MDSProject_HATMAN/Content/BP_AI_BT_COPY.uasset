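; Hatman enemy AI that hunts the player, ending in a forced look-at jumpscare, game over and level reload on capture.
; Event-graph AIMoveTo chains drive roaming, noise investigation, sight chases and timed runs to the player's position unless hidden.
; PawnSensing and AIPerception feed movement; hiding events toggle PawnSensing, and teleports boost speed and senses while shortening the timer.
; Also includes a cooldown-gated stun and finishes a BP_Test_AI_Bug test on capture.
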(event `AI can sense player`
  ;[0 0 0] AI can sense the player since he's not hiding.
  (set `PawnSensingComponent.bSeePawns` true (`self.PawnSensing`))
  (set `PawnSensingComponent.bHearNoises` true (`self.PawnSensing`))
  (set `PawnSensingComponent.HearingThreshold` (`self.Last Hearing Threshold`) (`self.PawnSensing`))
  (set `PawnSensingComponent.LOSHearingThreshold` (`self.Last LOSHearing Threshold`) (`self.PawnSensing`))
  (set `PawnSensingComponent.SightRadius` (`self.Last Sight Radius`) (`self.PawnSensing`)))

(event `AI cannot sense player`
  ;[0 0 0] AI cannot sense the player anymore because player is currently hiding.
  (set `PawnSensingComponent.HearingThreshold` 0.0 (`self.PawnSensing`))
  (set `PawnSensingComponent.LOSHearingThreshold` 0.0 (`self.PawnSensing`))
  (set `PawnSensingComponent.SightRadius` 0.0 (`self.PawnSensing`))
  (set `PawnSensingComponent.bSeePawns` false (`self.PawnSensing`))
  (set `PawnSensingComponent.bHearNoises` false (`self.PawnSensing`)))

(event `Teleported`
  ;[0 0 0] When AI teleports, it gets stronger (+ Store the updated PawnSensing Values in variables).
  (set `self.Speed` (+ (`self.Speed`) 100.0))
  (bind _output_get (set `PawnSensingComponent.HearingThreshold` (+ (`PawnSensingComponent.HearingThreshold` (`self.PawnSensing`)) 250.0) (`self.PawnSensing`)))
  (set `self.Last Hearing Threshold` _output_get)
  (bind _output_get_2 (set `PawnSensingComponent.LOSHearingThreshold` (+ (`PawnSensingComponent.LOSHearingThreshold` (`self.PawnSensing`)) 250.0) (`self.PawnSensing`)))
  (set `self.Last LOSHearing Threshold` _output_get_2)
  (bind _output_get_3 (set `PawnSensingComponent.SightRadius` (+ (`PawnSensingComponent.SightRadius` (`self.PawnSensing`)) 100.0) (`self.PawnSensing`)))
  (set `self.Last Sight Radius` _output_get_3)
  (set `self.Timer` (- (`self.Timer`) 5.0)))

(event `RunAI`
  ;[0.125 0.125 0.125 1 40] AI Running Function at a certain dynamic speed
  (if (not (`self.Caught?`)) :!pinned true
    (set `CharacterMovementComponent.MaxWalkSpeed` (`self.Speed`) (`self.CharacterMovement`) :!pinned true) ; Higher Groud Speed when running
  ))

(event `WalkAI`
  ;[0.08333 0.08333 0.08333 1 40] AI Walking Function at a certain dynamic speed
  (if (not (`self.Caught?`)) :!pinned true
    (set `CharacterMovementComponent.MaxWalkSpeed` (`self.Walking`) (`self.CharacterMovement`) :!pinned true) ; Lower Ground Speed when walking
  ))

(event `self.ReceiveBeginPlay`
  ;[0.1146 0.1146 0.1146 1 40] AI will wait 5 seconds before starting roaming when begin playing
  (`KismetSystemLibrary.RetriggerableDelay` 2.0) ; 2 seconds delay before Enemy AI starts roaming
  (`self.WalkAI`) ; AI is roaming (WalkAI Event triggered)
  (`self.CanSprintAgain`) ; AI starts running when seeing the player
  (`self.MoveToRandomLocation`) ; MoveToRandomLocation Event triggered
  (`GameplayStatics.SpawnSoundAttached` "/Game/SC_Hatman.SC_Hatman" (`self.CapsuleComponent`) "None" (0.0 0.0 0.0) (struct) "KeepRelativeOffset" false 1.0 1.0 0.0 null null))

(event `MoveToRandomLocation`
  ;[0.1042 0.1042 0.1042 1 40] Function which will make the AI move to a
  ; random location based on a given radius value (ex. 1000)
  (if (not (`self.Caught?`)) :!pinned true
    (`|AIMoveTo` self (`NavigationSystemV1.K2_GetRandomReachablePointInRadius` (`self.K2_GetActorLocation`) 1000.0 null null) null :!pinned true ; AI will move to the random reachable point previously generated
      (:`OnSuccess`
        (`KismetSystemLibrary.Delay` 1.5)
        (if (`self.Investigating?`) :!pinned true :!label _label
          (`|AIMoveTo` self (`self.Last_locations`) null :!pinned true ; AI will move to the last location set if it is still investigating
            (:`then`
              (`KismetSystemLibrary.RetriggerableDelay` 1.0)
              (`self.WalkAI` :!pinned true) ; Walk AI Event triggered
            )
            (:`OnSuccess`
              (set `self.Investigating?` false)
              (goto _label)))
          (else
            (`self.MoveToRandomLocation` :!pinned true :!label _label_2) ; MoveToRandomLocation Event triggered
            ;;[1 0.25 0 0.2 40] Every 30 seconds the AI will get the player's location on the map and will run towards that site,
            ;; before the AI will start roaming again (MoveToRandomLocation Event triggered)
            ;;
            ;; !!! Important: If the player is currently hiding, the AI will just roam around, until the player is no longer hiding.
            (`KismetSystemLibrary.Delay` (`self.Timer`) :!pinned true) ; Waiting time in seconds for the AI to be informed about the player's location
            (bind _asbp_third_person_character (cast `/Game/ThirdPerson/Blueprints/BP_ThirdPersonCharacter` (`GameplayStatics.GetPlayerCharacter` 0)))
            (if (`/Game/ThirdPerson/Blueprints/BP_ThirdPersonCharacter.playerHiding?` _asbp_third_person_character)
              (goto _label_2)
              (else
                (`|AIMoveTo` self (`SceneComponent.K2_GetComponentLocation` (`Actor.RootComponent` (`GameplayStatics.GetPlayerCharacter` 0))) null :!pinned true ; Enemy AI will move to the player's location
                  (:`then`
                    (`self.RunAI` :!pinned true) ; Enemy AI starts running towards player
                  )
                  (:`OnSuccess`
                    (goto _label_2))))))))
      (:`OnFail`
        (goto _label_2)))))

(event `self.PawnSensing.OnHearNoise`
  (params (Instigator :type "Pawn Object Reference") (Location :type "Vector Structure (by ref)") (Volume :type "Float (single-precision)"))
  ;[0.2656 0.2656 0.2656 1 40] Noise AI (walk on direction of the noise)
  (if (not (`self.Caught?`)) :!pinned true
    (bind _output_get (set `self.Last_locations` Location :!pinned true)) ; Update the last location vector to the noise coordinates on the map
    (`|AIMoveTo` self _output_get null :!pinned true ; AI will move to the last location previously updated
      (:`then`
        (set `self.Investigating?` true) ; AI is now investigating
        (`KismetSystemLibrary.RetriggerableDelay` 1.0)
        (`self.WalkAI` :!pinned true) ; AI is roaming (WalkAI Event triggered)
        (`self.CanSprintAgain`) ; CanSprintAgain Event triggered
        (`self.MoveToRandomLocation` :!pinned true) ; MoveToRandomLocation Event triggered
      ))))

(event `CanSprintAgain`
  ;[0.3229 0.3229 0.3229 1 40] When the Enemy AI sees the player, he starts running after him
  (goto _label_3 :!via `Reset`))

(event `self.PawnSensing.OnSeePawn`
  (params (Pawn :type "Pawn Object Reference"))
  ;[0.3229 0.3229 0.3229 1 40] When the Enemy AI sees the player, he starts running after him
  (if (not (`self.Caught?`))
    (`|ExecutionSequence`
      (:`then_0`
        (`/Engine/EditorBlueprintResources/StandardMacros.DoOnce` false :!label _label_3
          (:`Completed`
            (`self.RunAI`) ; RunAI Event triggered
          )))
      (:`then_1`
        (`|AIMoveTo` self (0.0 0.0 0.0) Pawn ; AI will move to the targeted player
          (:`then`
            (`KismetSystemLibrary.RetriggerableDelay` 1.0)
            (`self.WalkAI`) ; WalkAI Event triggered
            (`self.CanSprintAgain`) ; CanSprintAgain Event triggered
            (`self.MoveToRandomLocation`) ; MoveToRandomLocation Event triggered
          )
          (:`OnSuccess`
            (`self.Caught Player`) ; CaughtPlayer Event triggered
          ))))))

(event `Rotation Loop`
  ;[0.2712 0.517 0.6406 0.2 40] Enemy AI Animation + Restart Game when the AI entity catches the player -> GAME OVER ("Jumpscare" 2D Sound included)!
  (if (`self.Caught?`) :!label _label_4
    (`KismetSystemLibrary.Delay` 0.001)
    (bind _returnvalue (`KismetMathLibrary.FindLookAtRotation` (`self.K2_GetActorLocation` (stale `Caught Player` _asbp_third_person_character)) (`self.K2_GetActorLocation`)))
    (`self.K2_SetActorRotation` (stale `Caught Player` _asbp_third_person_character) _returnvalue false) ; Set the player's rotation instantly to the specified rotation
    (`Controller.SetControlRotation` (`GameplayStatics.GetPlayerController` 0) _returnvalue) ; Rotating the player towards the Enemy AI
    (`self.Rotation Loop`)
    (`/Engine/EditorBlueprintResources/StandardMacros.DoOnce` false
      (:`Completed`
        ;;[0 0 0 1 25] "JUMPSCARE" 2D Sound when player caught by AI.
        (`GameplayStatics.PlaySound2D` "/Game/Sound_Effects/HatmanJumpscare.HatmanJumpscare" 0.7 0.6 0.0 null null) ; "Jumpscare_Sound" played at 150% Volume
        (`KismetSystemLibrary.Delay` 1.0) ; '1' second delay
        ;;[1 1 1] Test AI Bug
        (bind _returnvalue_2 (`GameplayStatics.GetActorOfClass` "/Game/ThirdPerson/Blueprints/BP_Test_AI_Bug.BP_Test_AI_Bug_C"))
        (`FunctionalTest.FinishTest` _returnvalue_2 "Succeeded" "")
        (`PlayerCameraManager.StartCameraFade` :`self` (`GameplayStatics.GetPlayerCameraManager` 0) :`ToAlpha` 1.0 :`Duration` 2.0 :`bShouldFadeAudio` true :`bHoldWhenFinished` true) ; Fade the screen to black in 3 seconds
        (`KismetSystemLibrary.Delay` 0.5)
        (`self.GAME OVER`) ; Show GAME OVER Screen Text during Camera Fade Action
        (`KismetSystemLibrary.Delay` 3.0)
        (bind _returnvalue_3 (`GameplayStatics.GetCurrentLevelName` true)) ; Getting the currently-open Level
        (`GameplayStatics.OpenLevel` (`KismetStringLibrary.Conv_StringToName` _returnvalue_3)) ; The player travels back to the last checkpoint in the same Level
        (set `self.Caught?` false)))))

(event `Caught Player`
  ;[0.2712 0.517 0.6406 0.2 40] Enemy AI Animation + Restart Game when the AI entity catches the player -> GAME OVER ("Jumpscare" 2D Sound included)!
  (set `self.Caught?` true)
  (bind _asbp_third_person_character (cast `/Game/ThirdPerson/Blueprints/BP_ThirdPersonCharacter` (`GameplayStatics.GetPlayerCharacter` 0)))
  (goto _label_4))

(event `GAME OVER`
  ;[0.03154 0 0.1094 0.2 40] Adding the GAME OVER Screen Text (Widget BP)
  (bind _returnvalue (`|CreateWidget` "/Game/UI/Widget_Blueprints/GAME_OVER.GAME_OVER_C"))
  (`UserWidget.AddToViewport` _returnvalue 0) ; Adds the GAME OVER Widget to the game's viewport and fills the entire screen
  (bind _returnvalue_2 (`GameplayStatics.GetActorOfClass` "/Game/ThirdPerson/Blueprints/BP_ThirdPersonCharacter.BP_ThirdPersonCharacter_C"))
  (`CharacterMovementComponent.DisableMovement` (`Character.CharacterMovement` _returnvalue_2)))

(event `self.AIPerception.OnTargetPerceptionUpdated`
  (params (Actor :type "Actor Object Reference") (Stimulus :type "AIStimulus Structure"))
  (bind (_age _expirationage _strength _stimuluslocation _receiverlocation _tag _bsuccessfullysensed) (break `AIStimulus` Stimulus))
  ;[1 0.3 0 0.1 40] Distract the Enemy AI with noise.
  (cast `/Game/ThirdPerson/Blueprints/BP_ThirdPersonCharacter` Actor)
  (if _bsuccessfullysensed
    (set `self.Investigating?` true)
    (`|AIMoveTo` self _stimuluslocation null
      (:`OnSuccess`
        (`KismetSystemLibrary.Delay` 1.0)
        (`self.MoveToRandomLocation`)))))

(event `Detect Noise`
  (params (Location :type "Vector Structure"))
  (`KismetSystemLibrary.PrintString` "Enemy AI Detected NOISE " true true (struct :`G` 1.0 :`B` 0.278928 :`A` 1.0))
  (set `self.Investigating?` true)
  (`|AIMoveTo` self Location null
    (:`OnSuccess`
      (`KismetSystemLibrary.Delay` 1.0)
      (`self.MoveToRandomLocation`))))

(event `Aoleomamaochii`
  (`/Engine/EditorBlueprintResources/StandardMacros.DoOnce` false :!label _label_5
    (:`Completed`
      (`CharacterMovementComponent.DisableMovement` (`self.CharacterMovement`))
      (set `self.stunned` true)
      (`KismetSystemLibrary.Delay` 3.0)
      (`CharacterMovementComponent.SetMovementMode` (`self.CharacterMovement`) "MOVE_Swimming" 0)
      (set `self.stunned` false)
      (`KismetSystemLibrary.Delay` 20.0)
      (goto _label_5 :!via `Reset`))))

(fn `UserConstructionScript`)