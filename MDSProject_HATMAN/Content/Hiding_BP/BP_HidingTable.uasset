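; BP_HidingTable is a table the player can hide under from the AI.
; An outer trigger sets the player's crouch-to-hide prompt, while an inner trigger clears it and sets PlayerHiding.
; Entering or leaving the inner trigger calls AICannotSensePlayer or AICanSensePlayer on the BP_AI_BT found by GetActorOfClass, so only one AI is notified.
; Overlaps count only for the BP_ThirdPersonCharacter capsule, and debug prints remain.
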(event `self.TriggerIn.OnComponentBeginOverlap`
  (params (OverlappedComponent :type "PrimitiveComponent Object Reference") (OtherActor :type "Actor Object Reference") (OtherComp :type "PrimitiveComponent Object Reference") (OtherBodyIndex :type Integer) (bFromSweep :type Boolean) (SweepResult :type "HitResult Structure (by ref)"))
  ;[0 0 0] Player hiding from AI under the table.
  (bind _asbp_third_person_character (cast `/Game/ThirdPerson/Blueprints/BP_ThirdPersonCharacter` OtherActor))
  (if (== (`Character.CapsuleComponent` _asbp_third_person_character) OtherComp)
    (set `/Game/ThirdPerson/Blueprints/BP_ThirdPersonCharacter.Hiding Message` "" _asbp_third_person_character)
    (set `/Game/ThirdPerson/Blueprints/BP_ThirdPersonCharacter.playerHiding?` true _asbp_third_person_character)
    (bind _returnvalue (`GameplayStatics.GetActorOfClass` "/Game/AI/BP_AI_BT.BP_AI_BT_C"))
    (`/Game/AI/BP_AI_BT.AI cannot sense player` _returnvalue)
    (`KismetSystemLibrary.PrintString` "Hiding" true true (struct :`G` 1.0 :`A` 1.0)) ; TEST ONLY
  ))

(event `self.TriggerIn.OnComponentEndOverlap`
  (params (OverlappedComponent :type "PrimitiveComponent Object Reference") (OtherActor :type "Actor Object Reference") (OtherComp :type "PrimitiveComponent Object Reference") (OtherBodyIndex :type Integer))
  ;[0 0 0] Player hiding from AI under the table.
  (bind _asbp_third_person_character (cast `/Game/ThirdPerson/Blueprints/BP_ThirdPersonCharacter` OtherActor))
  (if (== (`Character.CapsuleComponent` _asbp_third_person_character) OtherComp)
    (set `/Game/ThirdPerson/Blueprints/BP_ThirdPersonCharacter.Hiding Message` "'Crouch' to Hide under the Table!" _asbp_third_person_character)
    (set `/Game/ThirdPerson/Blueprints/BP_ThirdPersonCharacter.playerHiding?` false _asbp_third_person_character)
    (bind _returnvalue (`GameplayStatics.GetActorOfClass` "/Game/AI/BP_AI_BT.BP_AI_BT_C"))
    (`/Game/AI/BP_AI_BT.AI can sense player` _returnvalue)
    (`KismetSystemLibrary.PrintString` "NOT Hiding" true true (struct :`R` 1.0 :`A` 1.0)) ; TEST ONLY
  ))

(event `self.TriggerOut.OnComponentBeginOverlap`
  (params (OverlappedComponent :type "PrimitiveComponent Object Reference") (OtherActor :type "Actor Object Reference") (OtherComp :type "PrimitiveComponent Object Reference") (OtherBodyIndex :type Integer) (bFromSweep :type Boolean) (SweepResult :type "HitResult Structure (by ref)"))
  ;[0 0 0] Screen Message warning the player that he can hide from AI under the table.
  (bind _asbp_third_person_character (cast `/Game/ThirdPerson/Blueprints/BP_ThirdPersonCharacter` OtherActor))
  (if (== (`Character.CapsuleComponent` _asbp_third_person_character) OtherComp)
    (set `/Game/ThirdPerson/Blueprints/BP_ThirdPersonCharacter.Hiding Message` "'Crouch' to Hide under the Table!" _asbp_third_person_character)))

(event `self.TriggerOut.OnComponentEndOverlap`
  (params (OverlappedComponent :type "PrimitiveComponent Object Reference") (OtherActor :type "Actor Object Reference") (OtherComp :type "PrimitiveComponent Object Reference") (OtherBodyIndex :type Integer))
  ;[0 0 0] No Screen Message warning the player that he can hide from AI anywhere.
  (bind _asbp_third_person_character (cast `/Game/ThirdPerson/Blueprints/BP_ThirdPersonCharacter` OtherActor))
  (if (== (`Character.CapsuleComponent` _asbp_third_person_character) OtherComp)
    (set `/Game/ThirdPerson/Blueprints/BP_ThirdPersonCharacter.Hiding Message` "" _asbp_third_person_character)))

(fn `UserConstructionScript`)