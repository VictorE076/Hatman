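; Enemy AI that roams random reachable points and hunts the player, scripted with AIMoveTo chains in the event graph.
; PawnSensing sight and noise redirect it, and a timer periodically sends it running to the player's position.
; Completing a sight or noise move triggers the catch: player turns to face it, game-over fade, level reload.
; Teleported events increase speed and senses and shorten the timer; throwable distraction is unfinished.
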(event `Teleported`
  ;[1 1 1] When AI teleports, it gets stronger
  (set `CharacterMovementComponent.MaxWalkSpeed` (+ (`CharacterMovementComponent.MaxWalkSpeed` (`self.CharacterMovement`)) 100.0) (`self.CharacterMovement`))
  (set `PawnSensingComponent.HearingThreshold` (+ (`PawnSensingComponent.HearingThreshold` (`self.PawnSensing`)) 250.0) (`self.PawnSensing`))
  (set `PawnSensingComponent.LOSHearingThreshold` (+ (`PawnSensingComponent.LOSHearingThreshold` (`self.PawnSensing`)) 250.0) (`self.PawnSensing`))
  (set `PawnSensingComponent.SightRadius` (+ (`PawnSensingComponent.SightRadius` (`self.PawnSensing`)) 100.0) (`self.PawnSensing`))
  (set `self.Timer` (- (`self.Timer`) 10.0)))

(event `RunAI`
  ;[0.125 0.125 0.125 1 40] AI Running Function at a given maximum speed (ex. 425)
  (if (not (`self.Caught?`)) :!pinned true
    (`SkeletalMeshComponent.PlayAnimation` (`self.Mesh`) "/Game/Characters/Mannequins/Animations/Manny/MM_Run_Fwd.MM_Run_Fwd" true) ; Animation for the AI Skeletal Mesh
    (set `CharacterMovementComponent.MaxWalkSpeed` 425.0 (`self.CharacterMovement`) :!pinned true) ; Higher Groud Speed when running
  ))

(event `WalkAI`
  ;[0.08333 0.08333 0.08333 1 40] AI Walking Function at a given maximum speed (ex. 170)
  (if (not (`self.Caught?`)) :!pinned true
    (`SkeletalMeshComponent.PlayAnimation` (`self.Mesh`) "/Game/Characters/Mannequins/Animations/Manny/MM_Walk_Fwd.MM_Walk_Fwd" true) ; Animation for the AI Skeletal Mesh
    (set `CharacterMovementComponent.MaxWalkSpeed` 170.0 (`self.CharacterMovement`) :!pinned true) ; Lower Ground Speed when walking
  ))

(event `self.ReceiveBeginPlay`
  ;[0.1146 0.1146 0.1146 1 40] AI will wait 5 seconds before starting roaming when begin playing
  (`KismetSystemLibrary.RetriggerableDelay` 5.0 :!pinned true) ; 5 seconds delay before Enemy AI starts roaming
  (`self.WalkAI` :!pinned true) ; AI is roaming (WalkAI Event triggered)
  (`self.CanSprintAgain`) ; AI starts running when seeing the player
  (`self.MoveToRandomLocation` :!pinned true) ; MoveToRandomLocation Event triggered
)

(event `MoveToRandomLocation`
  ;[0.1042 0.1042 0.1042 1 40] Function which will make the AI move to a
  ; random location based on a given radius value (ex. 1000)
  (if (not (`self.Caught?`)) :!pinned true
    (`|AIMoveTo` self (`NavigationSystemV1.K2_GetRandomReachablePointInRadius` (`self.K2_GetActorLocation`) 1000.0 null null) null :!pinned true ; AI will move to the random reachable point previously generated
      (:`OnSuccess`
        (`KismetSystemLibrary.Delay` 1.5)
        (if (`self.Investigating?`) :!pinned true :!label _label
          (`|AIMoveTo` self (`self.Last_locations`) null :!pinned true ; AI will move to the last location set if it is still investigating
            (:`then`
              (`KismetSystemLibrary.RetriggerableDelay` 1.0)
              (`self.WalkAI` :!pinned true) ; Walk AI Event triggered
            )
            (:`OnSuccess`
              (set `self.Investigating?` false)
              (goto _label)))
          (else
            (`self.MoveToRandomLocation` :!pinned true :!label _label_2) ; MoveToRandomLocation Event triggered
            ;;[0.06463 0.3854 0 0.2 40] Every 30 seconds the AI will get the player's location on the map and will run towards that site,
            ;; before the AI will start roaming again (MoveToRandomLocation Event triggered)
            (`KismetSystemLibrary.Delay` (`self.Timer`) :!pinned true) ; Waiting time in seconds for the AI to be informed about the player's location
            (`|AIMoveTo` self (`SceneComponent.K2_GetComponentLocation` (`Actor.RootComponent` (`GameplayStatics.GetPlayerCharacter` 0))) null :!pinned true ; Enemy AI will move to the player's location
              (:`then`
                (`self.RunAI` :!pinned true) ; Enemy AI starts running towards player
              )
              (:`OnSuccess`
                (goto _label_2))))))
      (:`OnFail`
        (goto _label_2)))))

(event `self.PawnSensing.OnHearNoise`
  (params (Instigator :type "Pawn Object Reference") (Location :type "Vector Structure (by ref)") (Volume :type "Float (single-precision)"))
  ;[0.2656 0.2656 0.2656 1 40] Noise AI (walk on direction of the noise)
  (if (not (`self.Caught?`)) :!pinned true
    (bind _output_get (set `self.Last_locations` Location :!pinned true)) ; Update the last location vector to the noise coordinates on the map
    (`|AIMoveTo` self _output_get null :!pinned true ; AI will move to the last location previously updated
      (:`then`
        (set `self.Investigating?` true) ; AI is now investigating
        (`KismetSystemLibrary.RetriggerableDelay` 1.0)
        (`self.WalkAI` :!pinned true) ; AI is roaming (WalkAI Event triggered)
        (`self.CanSprintAgain`) ; CanSprintAgain Event triggered
        (`self.MoveToRandomLocation` :!pinned true) ; MoveToRandomLocation Event triggered
      )
      (:`OnSuccess`
        (`self.Caught Player` :!pinned true) ; CaughtPlayer Event triggered
      ))))

(event `CanSprintAgain`
  ;[0.3229 0.3229 0.3229 1 40] When the Enemy AI sees the player, he starts running after him
  (goto _label_3 :!via `Reset`))

(event `self.PawnSensing.OnSeePawn`
  (params (Pawn :type "Pawn Object Reference"))
  ;[0.3229 0.3229 0.3229 1 40] When the Enemy AI sees the player, he starts running after him
  (if (not (`self.Caught?`))
    (`|ExecutionSequence`
      (:`then_0`
        (`/Engine/EditorBlueprintResources/StandardMacros.DoOnce` false :!label _label_3
          (:`Completed`
            (`self.RunAI` :!pinned true) ; RunAI Event triggered
          )))
      (:`then_1`
        (`|AIMoveTo` self (0.0 0.0 0.0) Pawn :!pinned true ; AI will move to the targeted player
          (:`then`
            (`KismetSystemLibrary.RetriggerableDelay` 1.0)
            (`self.WalkAI` :!pinned true) ; WalkAI Event triggered
            (`self.CanSprintAgain`) ; CanSprintAgain Event triggered
            (`self.MoveToRandomLocation` :!pinned true) ; MoveToRandomLocation Event triggered
          )
          (:`OnSuccess`
            (`self.Caught Player` :!pinned true) ; CaughtPlayer Event triggered
          ))))))

(event `Rotation Loop`
  (bind _returnvalue (`GameplayStatics.GetPlayerController` 0))
  ;[0.2712 0.517 0.6406 0.2 40] Enemy AI Animation + Restart Game when the AI entity catches the player -> GAME OVER!
  (if (`self.Caught?`) :!label _label_4
    (`KismetSystemLibrary.Delay` 0.001)
    (bind _returnvalue_2 (`KismetMathLibrary.FindLookAtRotation` (`self.K2_GetActorLocation` (stale `Caught Player` _asbp_third_person_character)) (`self.K2_GetActorLocation`)))
    (`self.K2_SetActorRotation` (stale `Caught Player` _asbp_third_person_character) (`KismetMathLibrary.RInterpTo` (`self.K2_GetActorRotation` (stale `Caught Player` _asbp_third_person_character)) _returnvalue_2 (`GameplayStatics.GetWorldDeltaSeconds`) 5.0) false) ; Set the player's rotation instantly to the specified rotation
    (`Controller.SetControlRotation` _returnvalue (`KismetMathLibrary.RInterpTo` (`Controller.GetControlRotation` _returnvalue) _returnvalue_2 (`GameplayStatics.GetWorldDeltaSeconds`) 5.0) :!pinned true) ; Rotating the player towards the Enemy AI
    (`self.Rotation Loop`)
    (`/Engine/EditorBlueprintResources/StandardMacros.DoOnce` false
      (:`Completed`
        (`SkeletalMeshComponent.PlayAnimation` (`self.Mesh`) "/Game/Paired_PushShove_Att_Montage.Paired_PushShove_Att_Montage" false) ; PushShove Animation playing once
        (`GameplayStatics.PlaySound2D` "/Game/Sound_Effects/GAME_OVER.GAME_OVER" 1.0 1.0 0.0 null null) ; "GAME OVER!" Sound
        (`PlayerCameraManager.StartCameraFade` :`self` (`GameplayStatics.GetPlayerCameraManager` 0) :`ToAlpha` 1.0 :`Duration` 3.0 :`bShouldFadeAudio` true :`bHoldWhenFinished` true) ; Fade the screen to black in 3 seconds
        (`KismetSystemLibrary.Delay` 1.25)
        (`SkeletalMeshComponent.PlayAnimation` (`self.Mesh`) "/Game/Characters/Mannequins/Animations/Manny/MM_Idle.MM_Idle" true) ; Idle Animation playing multiple times (Enemy AI stays still)
        (`self.GAME OVER` :!pinned true) ; Show GAME OVER Screen Text during Camera Fade Action
        (`KismetSystemLibrary.Delay` 4.0)
        (bind _returnvalue_3 (`GameplayStatics.GetCurrentLevelName` true)) ; Getting the currently-open Level
        (`GameplayStatics.OpenLevel` (`KismetStringLibrary.Conv_StringToName` _returnvalue_3) :!pinned true) ; The player travels back to the last checkpoint in the same Level
        (set `self.Caught?` false)))))

(event `Caught Player`
  ;[0.2712 0.517 0.6406 0.2 40] Enemy AI Animation + Restart Game when the AI entity catches the player -> GAME OVER!
  (set `self.Caught?` true)
  (bind _asbp_third_person_character (cast `/Game/ThirdPerson/Blueprints/BP_ThirdPersonCharacter` (`GameplayStatics.GetPlayerCharacter` 0)))
  (goto _label_4))

(event `GAME OVER`
  ;[0.03154 0 0.1094 0.2 40] Adding the GAME OVER Screen Text (Widget BP)
  (bind _returnvalue (`|CreateWidget` "/Game/UI/Widget_Blueprints/GAME_OVER.GAME_OVER_C"))
  (`UserWidget.AddToViewport` _returnvalue 0 :!pinned true) ; Adds the GAME OVER Widget to the game's viewport and fills the entire screen
)

(event `self.AIPerception.OnTargetPerceptionUpdated`
  (params (Actor :type "Actor Object Reference") (Stimulus :type "AIStimulus Structure"))
  ;[1 0 0 0.1 40] !!! Distract the Enemy AI with noise (A_Throwable Object - NOT WORKING)
)

(fn `UserConstructionScript`)