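; Enemy AI character that chases the player and makes melee attacks once its PawnSensing component sees a pawn.
; Each sighting runs AI MoveTo toward the player, while Tick halts movement until the first sighting.
; On arrival it plays a random punch or shove montage and a sound, then runs a debug-drawn multi line trace whose hits are unused.
; The montage length serves as the attack cooldown.
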(event `self.ReceiveTick`
  (params (DeltaSeconds :type "Float (single-precision)"))
  (if (not (`self.isSeeingPlayer?`))
    (`MovementComponent.StopMovementImmediately` (`self.CharacterMovement`))))

(event `self.PawnSensing.OnSeePawn`
  (params (Pawn :type "Pawn Object Reference"))
  (set `self.isSeeingPlayer?` true)
  (`self.FollowPlayer`))

(event `FollowPlayer`
  (set `self.canAttack?` true)
  (if (`self.isSeeingPlayer?`)
    (`|AIMoveTo` self (0.0 0.0 0.0) (`GameplayStatics.GetPlayerCharacter` 0) 70.0
      (:`OnSuccess`
        (if (`self.canAttack?`)
          (set `self.canAttack?` false)
          ;[0.5581 0.6685 1] Random - Pounch / Push Animation Montage
          (`self.Random Animation`)
          ;[0.4618 1 0.8693] Random Choice Punch 1 / 2 Sound
          (`GameplayStatics.PlaySoundAtLocation` "/Game/Sound_Effects/PunchSoundCue.PunchSoundCue" (`self.K2_GetActorLocation`) (struct) 1.0 1.0 0.0 null null null null)
          (`KismetSystemLibrary.LineTraceMulti` :`Start` (`SceneComponent.GetSocketLocation` (`self.StartAttack`) "None") :`End` (`SceneComponent.GetSocketLocation` (`self.EndAttack`) "None") :`TraceChannel` "TraceTypeQuery1" :`DrawDebugType` "ForDuration")
          (`KismetSystemLibrary.Delay` (`self.delayDuration`))
          (set `self.canAttack?` true))))
    (else
      (set `self.isSeeingPlayer?` false))))

(event `Random Animation`
  ;[0.5581 0.6685 1] Random - Pounch / Push Animation Montage
  (set `self.attackNum` (`KismetMathLibrary.RandomIntegerInRange` 0 1))
  (if (== (`self.attackNum`) 0)
    (bind _returnvalue (`self.PlayAnimMontage` "/Game/Paired_CounterPunch_PalmStrike_Att_UE5_Montage.Paired_CounterPunch_PalmStrike_Att_UE5_Montage"))
    (set `self.delayDuration` _returnvalue)
    (elif (== (`self.attackNum`) 1)
      (bind _returnvalue_2 (`self.PlayAnimMontage` "/Game/Paired_PushShove_Att_Montage.Paired_PushShove_Att_Montage"))
      (set `self.delayDuration` _returnvalue_2))))

(fn `UserConstructionScript`)