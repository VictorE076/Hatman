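; Enemy AI character that roams, chases seen pawns and moves toward noises, scripted in the event graph without a behavior tree.
; Roaming chains random reachable-point moves until Investigating is set.
; PawnSensing triggers a DoOnce-gated run or a move to noise, with retriggerable delays restoring walking and roaming after stimuli stop.
; AIPerception sets Investigating, never cleared here, for a distraction move marked as not working.
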(event `RunAI`
  ;[0.125 0.125 0.125 1 30] AI Running Function at a given maximum speed (ex. 425)
  (`SkeletalMeshComponent.PlayAnimation` (`self.Mesh`) "/Game/Characters/Mannequins/Animations/Manny/MM_Run_Fwd.MM_Run_Fwd" true)
  (set `CharacterMovementComponent.MaxWalkSpeed` 425.0 (`self.CharacterMovement`)))

(event `WalkAI`
  ;[0.08333 0.08333 0.08333 1 30] AI Walking Function at a given maximum speed (ex. 170)
  (`SkeletalMeshComponent.PlayAnimation` (`self.Mesh`) "/Game/Characters/Mannequins/Animations/Manny/MM_Walk_Fwd.MM_Walk_Fwd" true)
  (set `CharacterMovementComponent.MaxWalkSpeed` 170.0 (`self.CharacterMovement`)))

(event `self.ReceiveBeginPlay`
  ;[0.1146 0.1146 0.1146 1 30] AI will wait 5 seconds before starting roaming when begin playing
  (`KismetSystemLibrary.RetriggerableDelay` 5.0)
  (`self.WalkAI`)
  (`self.CanSprintAgain`)
  (`self.MoveToRandomLocation`))

(event `MoveToRandomLocation`
  ;[0.1042 0.1042 0.1042 1 30] Function which will make the AI move to a
  ; random location based on a given radius value (ex. 1000)
  (`|AIMoveTo` self (`NavigationSystemV1.K2_GetRandomReachablePointInRadius` (`self.K2_GetActorLocation`) 1000.0 null null) null
    (:`OnSuccess`
      (`KismetSystemLibrary.Delay` 1.5)
      (if (not (`self.Investigating?`))
        (`self.MoveToRandomLocation` :!label _label)))
    (:`OnFail`
      (goto _label))))

(event `CanSprintAgain`
  ;[0.3229 0.3229 0.3229 1 30] When the Enemy AI sees us, he starts running after us
  (goto _label_2 :!via `Reset`))

(event `self.PawnSensing.OnSeePawn`
  (params (Pawn :type "Pawn Object Reference"))
  ;[0.3229 0.3229 0.3229 1 30] When the Enemy AI sees us, he starts running after us
  (`|ExecutionSequence`
    (:`then_0`
      (`/Engine/EditorBlueprintResources/StandardMacros.DoOnce` false :!label _label_2
        (:`Completed`
          (`self.RunAI`))))
    (:`then_1`
      (`|AIMoveTo` self (0.0 0.0 0.0) Pawn
        (:`then`
          (`KismetSystemLibrary.RetriggerableDelay` 1.0)
          (`self.WalkAI`)
          (`self.CanSprintAgain`)
          (`self.MoveToRandomLocation`))))))

(event `self.PawnSensing.OnHearNoise`
  (params (Instigator :type "Pawn Object Reference") (Location :type "Vector Structure (by ref)") (Volume :type "Float (single-precision)"))
  ;[0.2656 0.2656 0.2656 1 30] Noise AI (walk on direction of the noise)
  (`KismetSystemLibrary.PrintString` (`KismetSystemLibrary.GetDisplayName` Instigator))
  (`|AIMoveTo` self Location null
    (:`then`
      (`KismetSystemLibrary.RetriggerableDelay` 1.0)
      (`self.WalkAI`)
      (`self.CanSprintAgain`)
      (`self.MoveToRandomLocation`))))

(event `self.AIPerception.OnTargetPerceptionUpdated`
  (params (Actor :type "Actor Object Reference") (Stimulus :type "AIStimulus Structure"))
  (bind (_age _expirationage _strength _stimuluslocation _receiverlocation _tag _bsuccessfullysensed) (break `AIStimulus` Stimulus))
  ;[0 0 0 1 30] Distract the Enemy AI with noise (A_Throwable Object - not working)
  (if _bsuccessfullysensed
    (set `self.Investigating?` true)
    (`|AIMoveTo` self _stimuluslocation null
      (:`OnSuccess`
        (`KismetSystemLibrary.PrintString` "Enemy AI Detected " true true (struct :`G` 1.0 :`B` 0.278928 :`A` 1.0))
        (`KismetSystemLibrary.RetriggerableDelay` 1.0)
        (`self.MoveToRandomLocation`)))))

(event `self.AIPerception.OnPerceptionUpdated`
  (params (UpdatedActors :type "Array of Actor Object Reference (by ref)")))

(fn `UserConstructionScript`)